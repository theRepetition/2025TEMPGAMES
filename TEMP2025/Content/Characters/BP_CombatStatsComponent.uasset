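; BP_CombatStatsComponent is a character component that tracks whether its owner is in combat.
; The enter-combat function (전투진입) adds the given actor to a set and raises the in-combat flag (전투중).
; The exit-combat function (전투해제) removes the actor and clears the flag only once the set is empty.
; The update and exit-check functions are empty stubs, and BeginPlay and Tick do nothing.
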(fn `전투 갱신`)

(fn `전투 진입`
  (params (`전투 진입한 액터` :type "Actor Object Reference (by ref)"))
  (`BlueprintSetLibrary.Set_Add` (`self.전투 해제확인 변수`) `전투 진입한 액터`)
  (if (not (`self.전투중`))
    (set `self.전투중` true)))

(fn `전투 해제`
  (params (`전투 해제할 액터` :type "Actor Object Reference"))
  (bind `_전투_해제확인_변수` (`self.전투 해제확인 변수`))
  (`BlueprintSetLibrary.Set_Remove` `_전투_해제확인_변수` `전투 해제할 액터`)
  (if (`BlueprintSetLibrary.Set_IsEmpty` `_전투_해제확인_변수`)
    (set `self.전투중` false)))

(fn `전투 해제 체크 함수`)