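; AI controller for BP_BaseNPC characters that issues patrol and enemy-chase movement orders.
; On BeginPlay it caches the controlled NPC and AI이동 sends it to the patrol point at the NPC's current index.
; 적추적 moves toward a given enemy using attack range as acceptance radius, returning one NPC state when already there and another when the request succeeds.
; Nothing here advances the patrol index or calls the chase.
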(event `self.ReceiveBeginPlay`
  (bind _asbp_base_npc (cast `/Game/Characters/NPC/BP_BaseNPC` (`self.K2_GetPawn`)))
  (set `self.ControlledNPC` _asbp_base_npc)
  (`self.AI이동`))

(event `self.ReceivePossess`
  (params (PossessedPawn :type "Pawn Object Reference")))

(fn `AI이동`
  (bind _controllednpc (`self.ControlledNPC`))
  (`self.MoveToActor` (`|GetArrayItem` (`/Game/Characters/NPC/BP_BaseNPC.순찰지점` _controllednpc) (`/Game/Characters/NPC/BP_BaseNPC.현재 순찰지점 인덱스` _controllednpc)) -1.0 true true true null))

(fn `UserConstructionScript`)

(fn `적 추적`
  (params (`추적할 적` :type "Actor Object Reference") (`공격 범위` :type "Float (double-precision)"))
  (returns (NewParam :type "/Game/Characters/NPC/ENPCSTATE Enum"))
  (set `self.npc 상태` "NewEnumerator4")
  (bind _returnvalue (`self.MoveToActor` `추적할 적` `공격 범위` true true true null))
  (switch `EPathFollowingRequestResult` _returnvalue
    (:`AlreadyAtGoal`
      (set `self.npc 상태` "NewEnumerator2"))
    (:`RequestSuccessful`
      (set `self.npc 상태` "NewEnumerator4")))
  (return (`self.npc 상태`)))