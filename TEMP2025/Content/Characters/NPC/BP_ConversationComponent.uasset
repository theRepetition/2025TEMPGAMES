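; NPC conversation component that looks up an NPC's dialogue lines and, for now, prints them as debug strings.
; 대화시작 (start conversation) proceeds only when the player relationship value is non-negative, then calls 대화문캐싱 (cache dialogue) with the NPC name.
; That function scans every data table row and appends NPCID matches to the 캐싱 array, which is never cleared here, before each cached DialogueText is printed.
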(fn `대화문 캐싱`
  (params (`npc이름` :type String))
  (bind `_데이터테이블` (`self.데이터테이블`))
  (bind _outrownames (`DataTableFunctionLibrary.GetDataTableRowNames` `_데이터테이블`))
  (for _array_element _outrownames
    (bind _returnvalue (`|GetDataTableRow` `_데이터테이블` _array_element)
      (:`then`
        (if (== (`.NPCID_9_141E66564E807D91FB8648BF4FAC6E0B` (break `/Game/DataTable/bp_DataStruct` _returnvalue)) `npc이름`)
          (`KismetArrayLibrary.Array_Add` (`self.캐싱`) _returnvalue)
          (`KismetSystemLibrary.PrintString` "캐싱성공"))))))

(fn `대화시작`
  (params (`플레이어와의 관계도` :type Integer) (`NPC 이름` :type String))
  ;[1 1 1] 1.플레이어와의 관계도 체크
  ; 0보다 높거나 같을때만 대화 가능
  (if (>= `플레이어와의 관계도` 0)
    ;[1 1 1] 2.데이터 캐싱, NPC에 맞는 대화 지문 가져오기
    ; 해당 NPC가 긴 대화 지문 있는지도 체크
    (`self.대화문 캐싱` `NPC 이름`)
    (for _array_element (`self.캐싱`)
      (`KismetSystemLibrary.PrintString` (`KismetTextLibrary.Conv_TextToString` (`.DialogueText_8_D33C989548543C585E4633B87F806467` (break `/Game/DataTable/bp_DataStruct` _array_element)))))))