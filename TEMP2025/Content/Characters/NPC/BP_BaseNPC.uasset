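; Base NPC character that initializes profile, weapon and stats from the NPC data table by ID and delegates behavior to components.
; Incoming attacks resolve in the combat component and lower player relationship; death applies a larger penalty and spawns a lootable corpse carrying the inventory.
; Player interaction shows conversation lines in a speech widget timed by text length.
; Overlapping players start a looping head-socket line-trace timer that flags visible targets.
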(event `self.ReceiveBeginPlay`
  (bind _bp_profilecomponent (`self.BP_ProfileComponent`))
  (bind _asbp_game_instance (cast `/Game/0_Game/BP_GameInstance` (`GameplayStatics.GetGameInstance`)))
  (`self.사망처리 디스패처 바인드`)
  (set `self.인스턴스` _asbp_game_instance)
  (set `CharacterMovementComponent.MaxWalkSpeed` 200.0 (`self.CharacterMovement`))
  ;[1 1 1] npc 대화 지문 ui collapsed
  (set `Widget.Visibility` "Collapsed" (`WidgetComponent.GetUserWidgetObject` (`self.간단한대화위젯컴포넌트`)))
  ;[1 1 1] NPC 데이터 가져오기
  (bind _returnvalue (`|GetDataTableRow` "/Game/DataTable/DT_NPCDataTable.DT_NPCDataTable" (`self.NPCID`))
    (:`then`
      (set `self.NPC 정보` _returnvalue)
      (set `/Game/FirstPerson/Blueprints/BP_ProfileComponent.프로필` (struct) _bp_profilecomponent)
      (`/Game/FirstPerson/Blueprints/BP_ProfileComponent.변수 가져오기` _bp_profilecomponent (`self.무기오른손`) null)
      (`/Game/FirstPerson/Blueprints/BP_ProfileComponent.아이템 장착` _bp_profilecomponent)
      (bind (`_이름` `_npc스탯` `_npc공격스탯`) (break `/Game/DataTable/NPCProfileStruct` (`.프로필_36_13DB892B4D4011EC0C505391BF64D0E1` (break `/Game/DataTable/bp_NpcStruct` _returnvalue))))
      (set `self.Name` (`KismetTextLibrary.Conv_TextToString` `_이름`))
      (`/Game/Characters/Actions/BP_StatsComponent.초기 능력치지정_NPC용` (`self.BP_StatsComponent`) `_npc공격스탯` `_npc스탯`))))

(event `/Game/Characters/Actions/BPI_AttackNotify.EndAttack`
  (params (`공격자` :type "Actor Object Reference"))
  (`/Game/Characters/Actions/BpAttackComponent.공격 방향 회전 종료` (`self.BpAttackComponent`)))

(event `/Game/Characters/NPC/BPI_ATKTO.ATKTOACTOR`
  (params (`공격구조체` :type "/Game/FirstPerson/Blueprints/Attack/bp_ATKSTRucture Structure") (`공격자` :type "Actor Object Reference"))
  (bind _bp_relationcomponent (`self.BP_relationComponent`))
  ;[1 1 1] 피해 입는 판정
  (set `self.최종적으로 받은 공격구조체` `공격구조체`)
  (bind `_피해_받음` (`/Game/Characters/NPC/BP_CombatCOmponent.공격 받음 처리` (`self.BP_CombatCOmponent`) (`self.방어기능 상태`) (`self.공격방향체크용`) `공격구조체` `공격자`))
  (if `_피해_받음`
    (if (`KismetSystemLibrary.IsValid` _bp_relationcomponent)
      ;; 나중에 한두번 정도 때리는건 관계도 안까이게 만들어야 함 - 실수로 공격하는거 방지
      (`/Game/Characters/NPC/BP_relationComponent.개인 관계도 변동과 그에따른 팩션 관계도 변경` _bp_relationcomponent -10))))

(event `사망 처리`
  (bind _bp_inventorycomponent (`self.BP_inventoryCOmponent`))
  ;[1 1 1] 사망 처리후 시체 파밍
  (bind _returnvalue (`|SpawnActorFromClass` "/Game/World/BP_corpse.BP_corpse_C" (`SceneComponent.GetSocketTransform` (`self.Mesh`) "Root" "RTS_World") "AdjustIfPossibleButAlwaysSpawn" "MultiplyWithRoot" null null))
  (`/Game/FirstPerson/Blueprints/BP_inventoryCOmponent.사망시 아이템 처리` _bp_inventorycomponent)
  (`/Game/World/BP_corpse.InitializeFromNPC` _returnvalue (`self.Mesh`) (`self.Name`) (`/Game/FirstPerson/Blueprints/BP_ContainerComponents.인벤토리` _bp_inventorycomponent) (`/Game/FirstPerson/Blueprints/BP_ContainerComponents.인벤토리 X 넓이` _bp_inventorycomponent) (`/Game/FirstPerson/Blueprints/BP_ContainerComponents.인벤토리 Y 높이` _bp_inventorycomponent) (`/Game/FirstPerson/Blueprints/BP_ContainerComponents.인벤토리 인덱스` _bp_inventorycomponent) (`/Game/FirstPerson/Blueprints/BP_ContainerComponents.엔트리 ID 발급용 인트` _bp_inventorycomponent))
  (`/Game/FirstPerson/Blueprints/BP_ContainerComponents.모든 아이템 내보내기` _bp_inventorycomponent)
  (`/Game/Characters/NPC/BP_relationComponent.개인 관계도 변동과 그에따른 팩션 관계도 변경` (`self.BP_relationComponent`) -100)
  (`self.K2_DestroyActor`)
  (set `self.사망처리` true))

(event `/Game/Characters/Actions/BPI_NPCInteraction.PlayertoNPC`
  (params (NewParam :type "/Game/Characters/Actions/STR_PlayerToNPC Structure"))
  (bind ((`PlayerName_2_390AC25E46065626068AE2B73A4B1767` _playername) (`Test_str_5_AE4C778040A4B479EC0AFF8EA8FF535A` _test_str)) (break `/Game/Characters/Actions/STR_PlayerToNPC` NewParam))
  (`cppNPCInteraction.ProcessPlayerStateWithValue` (`self.cppNPCInteraction`) _playername _test_str 0)
  (bind `_출력_짧은_대화문` (`/Game/Characters/NPC/BP_ConversationComponent.대화시작` (`self.BP_ConversationComponent`) 0 (`self.Name`) (`self.긴대화지문가지고있음`) "NewEnumerator0"))
  ;[1 1 1] 사망 처리후 시체 파밍
  (`self.간단한 대화문 출력` (`KismetTextLibrary.Conv_StringToText` `_출력_짧은_대화문`)))

(event `간단한 대화문 출력`
  (params (`간단한 대화문 텍스트 입력` :type Text))
  (bind _returnvalue (`WidgetComponent.GetUserWidgetObject` (`self.간단한대화위젯컴포넌트`)))
  (bind _aswbp_speech_box (cast `/Game/UI/WBP_SpeechBox` _returnvalue))
  (`/Game/UI/WBP_SpeechBox.set짧은대화지문` _aswbp_speech_box `간단한 대화문 텍스트 입력`)
  (`Widget.SetVisibility` _returnvalue "Visible")
  (`KismetSystemLibrary.Delay` (+ (* (`self.NewVar`) (`KismetStringLibrary.Len` (`KismetTextLibrary.Conv_TextToString` `간단한 대화문 텍스트 입력`))) 2.0))
  (`Widget.SetVisibility` _returnvalue "Collapsed"))

(event `self.액터 감지용.OnComponentBeginOverlap`
  (params (OverlappedComponent :type "PrimitiveComponent Object Reference") (OtherActor :type "Actor Object Reference") (OtherComp :type "PrimitiveComponent Object Reference") (OtherBodyIndex :type Integer) (bFromSweep :type Boolean) (SweepResult :type "HitResult Structure (by ref)"))
  (if (`self.ActorHasTag` OtherActor "Player")
    ; 라인 트레이스 전 후보 올리기
    ;
    ; 후보와 NPC 사이에 시야가막혀 있지 않다면 추적대상
    (set `self.추적 후보` OtherActor)
    (`KismetSystemLibrary.K2_SetTimer` null "플레이어 추적" 0.2 true)))

(event `self.액터 감지용.OnComponentEndOverlap`
  (params (OverlappedComponent :type "PrimitiveComponent Object Reference") (OtherActor :type "Actor Object Reference") (OtherComp :type "PrimitiveComponent Object Reference") (OtherBodyIndex :type Integer))
  (if (`self.ActorHasTag` OtherActor "Player")
    (set `self.트레이스 체크` false)))

(fn `GetEOBJType`
  (params (OBJTYPE :type "EObjectType Enum" :default "None"))
  (returns (NewParam :type "EObjectType Enum"))
  (return (`self.OBJTYPE`)))

(fn `GetOBJName`
  (returns (name :type Text))
  (return (`KismetTextLibrary.Conv_StringToText` (`self.Name`))))

(fn `GUID-> 인스턴스-> DEF`
  (params (Guid :type "Guid Structure"))
  (returns (`아웃 행` :type "/Game/Items/Item_DEF Structure"))
  (bind `_인스턴스` (`self.인스턴스`))
  (if (`KismetGuidLibrary.IsValid_Guid` Guid)
    (if (`KismetSystemLibrary.IsValid` `_인스턴스`)
      (bind _value (`/Game/0_Game/BP_GameInstance.아이템 인스턴스 찾기` `_인스턴스` Guid))
      (bind _returnvalue (`|GetDataTableRow` "/Game/Items/DataTable_itemDEF.DataTable_itemDEF" (`.DEFID_11_BBFD4A2F4114CCEB3D5A81BB9B1C9124` (break `/Game/Items/Item_InstanceID` _value)))
        (:`then`
          (return _returnvalue)))
      (else
        (bind _asbp_game_instance (cast `/Game/0_Game/BP_GameInstance` (`GameplayStatics.GetGameInstance`)))
        (bind _value_2 (`/Game/0_Game/BP_GameInstance.아이템 인스턴스 찾기` _asbp_game_instance Guid))
        (bind _returnvalue_2 (`|GetDataTableRow` "/Game/Items/DataTable_itemDEF.DataTable_itemDEF" (`.DEFID_11_BBFD4A2F4114CCEB3D5A81BB9B1C9124` (break `/Game/Items/Item_InstanceID` _value_2)))
          (:`then`
            (return _returnvalue_2)))))))

(fn `UserConstructionScript`)

(fn `개인 관계도 변동과 그에따른 팩션 관계도 변경`
  (params (`변경할 개인 관계도` :type Integer))
  (set `self.플레이어와의 일시/개인 관계도` (+ (`self.플레이어와의 일시/개인 관계도`) `변경할 개인 관계도`)))

(fn `경직 상태로`
  (locals (`임시 걷기 속도 저장` :type "Float (single-precision)" :default 0.0) (`원래 속도 저장` :type "Float (single-precision)" :default 0.0))
  (`/Game/FirstPerson/Blueprints/BP_CharConditionCOmponent.경직 상태 진행` (`self.BP_CharConditionCOmponent`) 1.0))

(fn `대기 중`)

(fn `사망처리 디스패처 바인드`
  (add `/Game/Characters/Actions/BP_StatsComponent.사망처리` (`self.BP_StatsComponent`) (`|CreateDelegate` :!event `사망 처리`)))

(fn `순찰`)

(fn `아이템 인스턴스에 등록`
  (params (ID1 :type Name))
  (returns (NewParam1 :type "Guid Structure"))
  (locals (`아이템 ID` :type Name) (NewLocalVar :type "Guid Structure"))
  (bind _newlocalvar (`local.NewLocalVar`))
  ; 신규 아이템 등록
  (bind _asbp_game_instance (cast `/Game/0_Game/BP_GameInstance` (`GameplayStatics.GetGameInstance`)))
  (set `local.NewLocalVar` (`KismetGuidLibrary.NewGuid`))
  (`/Game/0_Game/BP_GameInstance.아이템 인스턴스 등록` _asbp_game_instance _newlocalvar (make `/Game/Items/Item_InstanceID` _newlocalvar ID1 1))
  (return _newlocalvar))

(fn `아이템 프로필 반복 체크용`
  (params (`입력아이템` :type "ItemData Structure") (Selection :type "EIsEquipped Enum" :default "None")))

(fn `이동속도 업데이트`
  (params (`NPC 이동속도` :type "Float (double-precision)"))
  (set `CharacterMovementComponent.MaxWalkSpeed` `NPC 이동속도` (`self.CharacterMovement`)))

(fn `재생된 몽타주 저장`
  (params (`재생중인 몽타주` :type "AnimMontage Object Reference"))
  (set `self.재생중인 몽타주` `재생중인 몽타주`))

(fn `플레이어 추적`
  (bind _returnvalue (`SceneComponent.GetSocketLocation` (`self.Mesh`) "head"))
  (bind (_outhit _returnvalue_2) (`KismetSystemLibrary.LineTraceSingle` :`Start` _returnvalue :`End` (+ _returnvalue (* (`KismetMathLibrary.Normal` (- (`self.K2_GetActorLocation` (`self.추적 후보`)) _returnvalue) 1.0) (2000.0 2000.0 2000.0))) :`TraceChannel` "TraceTypeQuery3" :`DrawDebugType` "ForDuration" :`TraceColor` (struct :`R` 1.0 :`B` 0.627234 :`A` 1.0)))
  (if _returnvalue_2
    (if (`self.ActorHasTag` (`.HitActor` (`GameplayStatics.BreakHitResult` _outhit)) "Player")
      (set `self.트레이스 체크` true)
      (set `self.후보를 대상으로` true)
      (`KismetSystemLibrary.PrintString` "발견")
      (else
        (set `self.트레이스 체크` false)))
    (else
      (set `self.트레이스 체크` false))))

(fn `행동양식`
  (switch `int` (`KismetMathLibrary.RandomInteger` 3)))