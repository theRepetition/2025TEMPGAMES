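; Base NPC character with data-table profile, inventory and faction, supporting dialogue, melee combat and lootable death.
; PlayertoNPC shows relationship-based lines in a timed speech-bubble widget; player hits lower faction standing through the GameInstance.
; Spotting the player starts an AI-controller chase that triggers attack montages in combat.
; Attacks step a Swingbox along precomputed directional arcs on a timer, hitting HitboxComponents, while death spawns a corpse carrying mesh, inventory and name.
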(event `self.ReceiveBeginPlay`
  (set `CharacterMovementComponent.MaxWalkSpeed` 200.0 (`self.CharacterMovement`))
  ;[1 1 1] npc 대화 지문 ui collapsed
  (set `Widget.Visibility` "Collapsed" (`WidgetComponent.GetUserWidgetObject` (`self.간단한대화위젯컴포넌트`)))
  ;[1 1 1] NPC 데이터 가져오기
  (bind _returnvalue (`|GetDataTableRow` "/Game/DataTable/DT_NPCDataTable.DT_NPCDataTable" (`self.NPCID`))
    (:`then`
      (bind _output_get (set `self.NPC 정보` _returnvalue))
      (bind (`_팩션` `_npc타입` `_클래스` `_아이템테이블` `_프로필`) (break `/Game/DataTable/bp_NpcStruct` _output_get))
      (bind _output_get_2 (set `self.프로필` `_프로필`))
      (set `self.NPC 인벤토리` `_아이템테이블`)
      (bind (_playername _level _righthand _lefthand _accessoryl _accessoryr _helmet _armor _deftype _playerfinalstat) (break `PlayerProfile` _output_get_2))
      (set `self.Name` _playername)
      (bind _output_get_3 (set `self.MaxHealth` (`KismetMathLibrary.Conv_IntToDouble` (`.HP` (break `FinalStatsStruct` _playerfinalstat)))))
      (set `self.Health` _output_get_3)
      (bind _returnvalue_2 (`|GetDataTableRow` "/Game/DataTable/DT_FAactionDataTable.DT_FAactionDataTable" `_팩션`)
        (:`then`
          (bind _output_get_4 (set `self.Faction` _returnvalue_2))
          ;;[1 1 1] 팩션 같은거 있을때만 인스턴스 관계도 수치 받아오기
          (bind _asbp_game_instance (cast `/Game/0_Game/BP_GameInstance` (`GameplayStatics.GetGameInstance`)))
          (for _array_element (`/Game/0_Game/BP_GameInstance.팩션` _asbp_game_instance)
            (if (== (`.팩션이름_9_0F6684564B773AA659EC06B9743BF796` (break `/Game/DataTable/bp_FactionStruct` _output_get_4)) (`.팩션이름_9_0F6684564B773AA659EC06B9743BF796` (break `/Game/DataTable/bp_FactionStruct` _array_element)))
              (set `self.Faction` _array_element))))))))

(event `self.ATKTOACTOR`
  (params (`공격구조체` :type "/Game/FirstPerson/Blueprints/Attack/bp_ATKSTRucture Structure") (`공격자` :type "Actor Object Reference"))
  (bind (`_기본데미지` `_공격타입` `_공격방향`) (break `/Game/FirstPerson/Blueprints/Attack/bp_ATKSTRucture` `공격구조체`))
  (bind _health (`self.Health`))
  (bind _faction (`self.Faction`))
  (set `self.피해 받았는지 체크` true)
  ;[1 1 1] 피해 입는 판정
  (`KismetSystemLibrary.PrintString` (`|GetEnumeratorNameAsString` `_공격방향`))
  (set `self.Health` (- _health `_기본데미지`))
  ;[1 1 1 1 12] 플레이어가 공격했으면 해당 팩션의 관계도를 낮추기
  ; 데이터를 건드는게 아니라
  ; 인스턴스하고 연결해서 인스턴스 내부의 현재 게임의 관계도를 설정해야함
  (cast `/Game/FirstPerson/Blueprints/BP_FirstPersonCharacter` `공격자`
    (:`then`
      (bind _asbp_game_instance (cast `/Game/0_Game/BP_GameInstance` (`GameplayStatics.GetGameInstance`)))
      (setmembers `/Game/DataTable/bp_FactionStruct` :`StructRef` _faction :`플레이어와의 관계 수치` (- (`.플레이어와의관계수치_6_56E833414AD9AE5DB1DCE088D8325AE9` (break `/Game/DataTable/bp_FactionStruct` _faction)) 1))
      (`/Game/0_Game/BP_GameInstance.팩션 관계도 감소` _asbp_game_instance _faction))
    (:`CastFailed`
      _))
  ;[1 1 1] 사망 처리후 시체 파밍
  (if (<= _health 0.0)
    (bind _returnvalue (`|SpawnActorFromClass` "/Game/World/BP_corpse.BP_corpse_C" (`SceneComponent.GetSocketTransform` (`self.Mesh`) "Root" "RTS_World") "AdjustIfPossibleButAlwaysSpawn" "MultiplyWithRoot" null null))
    (`/Game/World/BP_corpse.InitializeFromNPC` _returnvalue (`self.Mesh`) (`self.NPC 인벤토리`) (`self.Name`))
    (`self.K2_DestroyActor`)
    (set `self.사망처리` true)
    (else
      (`KismetSystemLibrary.Delay` 0.2)
      (set `self.피해 받았는지 체크` false))))

(event `self.PlayertoNPC`
  (params (NewParam :type "/Game/Characters/Actions/STR_PlayerToNPC Structure"))
  (bind (_playername _test_str) (break `/Game/Characters/Actions/STR_PlayerToNPC` NewParam))
  (`cppNPCInteraction.ProcessPlayerStateWithValue` (`self.cppNPCInteraction`) _playername _test_str 0)
  (bind `_출력_짧은_대화문` (`/Game/Characters/NPC/BP_ConversationComponent.대화시작` (`self.BP_ConversationComponent`) (`.플레이어와의관계수치_6_56E833414AD9AE5DB1DCE088D8325AE9` (break `/Game/DataTable/bp_FactionStruct` (`self.Faction`))) (`self.Name`) (`self.긴대화지문가지고있음`)))
  (`self.간단한 대화문 출력` (`KismetTextLibrary.Conv_StringToText` `_출력_짧은_대화문`)))

(event `간단한 대화문 출력`
  (params (`간단한 대화문 텍스트 입력` :type Text))
  (bind _returnvalue (`WidgetComponent.GetUserWidgetObject` (`self.간단한대화위젯컴포넌트`)))
  (bind _aswbp_speech_box (cast `/Game/UI/WBP_SpeechBox` _returnvalue))
  (`/Game/UI/WBP_SpeechBox.set짧은대화지문` _aswbp_speech_box `간단한 대화문 텍스트 입력`)
  (`Widget.SetVisibility` _returnvalue "Visible")
  (`KismetSystemLibrary.Delay` (+ (* (`self.NewVar`) (`KismetStringLibrary.Len` (`KismetTextLibrary.Conv_TextToString` `간단한 대화문 텍스트 입력`))) 2.0))
  (`Widget.SetVisibility` _returnvalue "Collapsed"))

(event `self.이동 감지.OnSeePawn`
  (params (Pawn :type "Pawn Object Reference"))
  ;[1 1 1] 플레이어 감지하면 형변환해서 ai컨트롤러 함수 써먹기
  (set `CharacterMovementComponent.MaxWalkSpeed` 400.0 (`self.CharacterMovement`))
  (if (`self.ActorHasTag` Pawn "Player")
    (set `self.추적 대상` Pawn)
    (bind _asbp_npccontroller (cast `/Game/Characters/NPC/BP_NPCController` (`AIBlueprintHelperLibrary.GetAIController` self)))
    (bind _output_get (set `self.NPC컨트롤러` _asbp_npccontroller))
    (bind _newparam (`/Game/Characters/NPC/BP_NPCController.적 추적` _output_get Pawn (- (`self.공격 범위`) 50.0)))
    (switch `/Game/Characters/NPC/ENPCSTATE` _newparam
      (:`NewEnumerator2`
        (`self.행동양식`)
        (if (not (`self.공격중`))
          (`|PlayMontage` (`self.Mesh`) "/Game/Sword_Animation/Animations/Montage/Montage_NpcAttack_upper.Montage_NpcAttack_upper"
            (:`then`
              (set `self.공격중` true)
              (`self.공격 방향 회전 시작_NPC`))
            (:`OnCompleted`
              (set `self.공격중` false))))))))

(fn `GetEOBJType`
  (params (OBJTYPE :type "EObjectType Enum" :default "None"))
  (returns (NewParam :type "EObjectType Enum"))
  (return (`self.OBJTYPE`)))

(fn `GetOBJName`
  (returns (name :type Text))
  (return (`KismetTextLibrary.Conv_StringToText` (`self.Name`))))

(fn `UserConstructionScript`)

(fn `공격 방향 회전 시작_NPC`
  (bind _swingbox (`self.Swingbox`))
  (`BlueprintSetLibrary.Set_Clear` (`self.피격컴포넌트세트`))
  (bind _output_get (set `self.현재단계` 0))
  (`self.공격 방향 회전 판별_NPC` (`self.공격방향체크용`))
  (`PrimitiveComponent.SetCollisionEnabled` _swingbox "QueryOnly")
  (`SceneComponent.K2_SetRelativeTransform` _swingbox (`|GetArrayItem` (`self.회전단계`) _output_get) false false)
  (bind _returnvalue (`KismetSystemLibrary.K2_SetTimer` null "공격 방향 회전 진행_NPC" 0.02 true))
  (set `self.공격측정타이머` _returnvalue))

(fn `공격 방향 회전 종료_NPC`
  (`KismetSystemLibrary.K2_ClearTimer` null "공격 방향 회전 진행_NPC")
  (`PrimitiveComponent.SetCollisionEnabled` (`self.Swingbox`) "NoCollision")
  (`BlueprintSetLibrary.Set_Clear` (`self.피격액터세트_0`))
  (set `self.현재단계` 0))

(fn `공격 방향 회전 진행_NPC`
  (bind `_피격액터세트_0` (`self.피격액터세트_0`))
  (bind `_현재단계` (`self.현재단계`))
  (bind `_회전단계` (`self.회전단계`))
  (for _array_element (`PrimitiveComponent.GetOverlappingComponents` (`self.Swingbox`))
    (bind _returnvalue (`ActorComponent.GetOwner` _array_element))
    ;[1 1 1] 세트에 존재하는지(이미 충돌했는지) 체크
    (if (not (== _returnvalue self))
      (cast `HitboxComponent` _array_element)
      (if (not (`BlueprintSetLibrary.Set_Contains` `_피격액터세트_0`))
        ;[1 1 1] 없으면(첫 충돌이면) 추가하고 데미지
        (`BlueprintSetLibrary.Set_Add` `_피격액터세트_0`)
        (`/Game/Characters/Actions/BpAttackComponent.AttackFromCompo` (`self.BpAttackComponent`) (`self.StaminaCost`) (`self.HitDamage`) (`self.BP_StaminaComponent`) (`KismetMathLibrary.Conv_IntToDouble` (`.SP` (break `FinalStatsStruct` (`.PlayerFinalStat` (break `PlayerProfile` (`self.프로필`)))))) self "NewEnumerator1" _returnvalue _array_element (`self.공격방향체크용`)))))
  (set `self.현재단계` (+ 1 `_현재단계`))
  (if (>= `_현재단계` (`KismetArrayLibrary.Array_Length` `_회전단계`))
    (`self.공격 방향 회전 종료_NPC`)
    (else
      (`SceneComponent.K2_SetRelativeTransform` (`self.Swingbox`) (`|GetArrayItem` `_회전단계` `_현재단계`) false false))))

(fn `공격 방향 회전 판별_NPC`
  (params (NewParam :type "EAttackDirection Enum" :default "None"))
  (locals (`시작각` :type "Float (double-precision)") (`최종각` :type "Float (double-precision)") (`회전각` :type "Float (double-precision)") (`좌우` :type "Vector Structure" :default (0.0 0.0 70.0)) (`액터포워드 각도` :type "Vector Structure" :default (0.0 0.0 20.0)))
  (bind _returnvalue (- (`self.각변화 단계`) 1))
  (switch `EAttackDirection` NewParam
    (:`Left`
      (`KismetSystemLibrary.PrintString` "왼쪽")
      (set `local.시작각` -90.0)
      (set `local.회전각` 15.0)
      (set `local.최종각` 20.0)
      (set `local.좌우` (0.0 -20.0 70.0))
      (set `local.액터포워드 각도` (0.0 0.0 5.0) :!label _label))
    (:`Right`
      (`KismetSystemLibrary.PrintString` "오른쪽")
      (set `local.시작각` 90.0)
      (set `local.회전각` 15.0)
      (set `local.최종각` -20.0)
      (set `local.좌우` (0.0 20.0 70.0))
      (goto _label))
    (:`Up`
      (set `local.시작각` -80.0)
      (set `local.회전각` 15.0)
      (set `local.최종각` 20.0)
      (set `local.좌우` (0.0 0.0 70.0))
      (set `local.액터포워드 각도` (0.0 5.0 0.0)))
    (:`Med`
      (set `local.시작각` 80.0)
      (set `local.회전각` 20.0)
      (set `local.최종각` 0.0)
      (set `local.좌우` (0.0 0.0 70.0))
      (set `local.액터포워드 각도` (0.0 5.0 0.0))))
  (`KismetArrayLibrary.Array_Clear` (`self.회전단계`))
  (for _index (range (+ _returnvalue 1))
    (bind _returnvalue_2 (`KismetMathLibrary.RotateAngleAxis` (`KismetMathLibrary.MakeVector` 6.0) (`KismetMathLibrary.Lerp` (`local.시작각`) (`local.최종각`) (/ (`KismetMathLibrary.Conv_IntToDouble` _index) (`KismetMathLibrary.Conv_IntToDouble` _returnvalue))) (`local.액터포워드 각도`)))
    (`KismetArrayLibrary.Array_Add` (`self.회전단계`) (`KismetMathLibrary.MakeTransform` (+ (* _returnvalue_2 (`local.회전각`)) (`local.좌우`)) (`KismetMathLibrary.MakeRotFromX` _returnvalue_2) (`SceneComponent.K2_GetComponentScale` (`self.Swingbox`))))))

(fn `공격/디버깅용`)

(fn `순찰`)

(fn `이동속도 업데이트`
  (params (`NPC 이동속도` :type "Float (double-precision)"))
  (set `CharacterMovementComponent.MaxWalkSpeed` `NPC 이동속도` (`self.CharacterMovement`)))

(fn `행동양식`
  (switch `int` (`KismetMathLibrary.RandomInteger` 3)))