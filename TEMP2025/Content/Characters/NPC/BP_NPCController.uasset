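; AI controller for BP_BaseNPC that runs NPC_BT on possess and handles chasing of a target the NPC has negative relations with.
; Tick focuses and follows the pawn's candidate target to attack range, backing away when too close and recording its last location.
; Losing trace starts two six-second timers: chasing continues, then moves to the last location, then drops the target unless the trace returns.
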(event `self.ReceiveBeginPlay`
  ; 사용안함
  (bind _asbp_base_npc (cast `/Game/Characters/NPC/BP_BaseNPC` (`self.K2_GetPawn`)))
  (set `self.ControlledNPC` _asbp_base_npc))

(event `self.ReceivePossess`
  (params (PossessedPawn :type "Pawn Object Reference"))
  ; BT 실행
  (bind _returnvalue (`self.RunBehaviorTree` "/Game/Characters/NPC/NPC_BT.NPC_BT"))
  (`KismetSystemLibrary.PrintString` (`KismetStringLibrary.Conv_BoolToString` _returnvalue)))

(event `self.ReceiveTick`
  (params (DeltaSeconds :type "Float (single-precision)"))
  (bind _returnvalue (`self.K2_GetPawn`))
  (bind `_추적할_npc` (`self.추적할 NPC`))
  (bind `_공격범위` (`self.공격범위`))
  (bind _returnvalue_2 (`self.K2_GetActorLocation` _returnvalue))
  (bind _returnvalue_3 (`self.K2_GetActorLocation` `_추적할_npc`))
  (bind _returnvalue_4 (`self.GetDistanceTo` `_추적할_npc` _returnvalue))
  (bind _returnvalue_5 (+ _returnvalue_2 (* (`KismetMathLibrary.Normal` (- _returnvalue_2 _returnvalue_3)) (75.0 75.0 0.0))))
  (bind _asbp_base_npc (cast `/Game/Characters/NPC/BP_BaseNPC` (`self.K2_GetPawn`)))
  ; 개인 관계도 낮지 않으면 굳이 추적 X
  (if (< (`/Game/Characters/NPC/BP_relationComponent.플레이어와의 일시/개인 관계도` (`/Game/Characters/NPC/BP_BaseNPC.BP_relationComponent` _asbp_base_npc)) 0)
    (if (`/Game/Characters/NPC/BP_BaseNPC.후보를 대상으로` _asbp_base_npc)
      (set `self.추적할 NPC` (`/Game/Characters/NPC/BP_BaseNPC.추적 후보` _asbp_base_npc))
      (if (`/Game/Characters/NPC/BP_BaseNPC.트레이스 체크` _asbp_base_npc)
        (set `self.아직은 추적가능` true)
        (set `self.최종적인 흔적 추적` true)
        (`self.K2_SetFocus` `_추적할_npc`)
        (if (< _returnvalue_4 `_공격범위`) :!label _label
          (if (< _returnvalue_4 (- (`self.공격범위`) 35.0))
            ; 너무 가까울때 후진
            (`self.MoveToLocation` _returnvalue_5 -1.0 true true false true null)
            (`KismetSystemLibrary.DrawDebugPoint` _returnvalue_5 20.0 (struct :`R` 1.0 :`G` 0.136865 :`B` 0.033996 :`A` 1.0))
            (set `self.마지막위치` _returnvalue_3 :!label _label_2))
          (else
            (`self.적 추적` `_공격범위`)
            (goto _label_2)))
        (else
          ; 트레이스 체크 불가 -> 벽있어서 못봄
          ; 그래도 n초동안 추적
          (if (`self.트레이스 변화 가능`)
            (`KismetSystemLibrary.K2_SetTimerDelegate` (delegate `1차 트레이스 체크`) 6.0 false true)
            (set `self.트레이스 변화 가능` false))
          (if (`self.아직은 추적가능`)
            (`self.K2_ClearFocus`)
            (goto _label)))))))

(event `1차 트레이스 체크`
  (bind `_마지막위치` (`self.마지막위치`))
  ; n초 뒤에도 트레이스 체크 못하는 상황
  (`KismetSystemLibrary.PrintString` "1차시도")
  (if (`/Game/Characters/NPC/BP_BaseNPC.트레이스 체크` (stale `self.ReceiveTick` _asbp_base_npc))
    (set `self.트레이스 변화 가능` true)
    (set `self.아직은 추적가능` true)
    (else
      (set `self.아직은 추적가능` false)
      ; 일단 안보이지만 플레이어 최종 위치로 이동 시도
      (`KismetSystemLibrary.PrintString` "1차 트레이스 실패")
      (`KismetSystemLibrary.K2_SetTimerDelegate` (delegate `2차 트레이스 체크`) 6.0 false true)
      (set `self.추적 종료 트리거` true)
      (`self.K2_ClearFocus`)
      (`KismetSystemLibrary.DrawDebugPoint` `_마지막위치` 20.0 (struct :`R` 0.598877 :`G` 0.971325 :`B` 1.0 :`A` 1.0))
      (bind _output_get (set `self.마지막위치_0` `_마지막위치`))
      (`self.MoveToLocation` _output_get 10.0 true true false true null))))

(event `2차 트레이스 체크`
  ; 최종적으로 트레이스 체크 못함
  (if (`/Game/Characters/NPC/BP_BaseNPC.트레이스 체크` (stale `self.ReceiveTick` _asbp_base_npc))
    (set `self.트레이스 변화 가능` true)
    (set `self.아직은 추적가능` true)
    (set `self.최종적인 흔적 추적` true)
    (else
      (set `/Game/Characters/NPC/BP_BaseNPC.후보를 대상으로` false (stale `self.ReceiveTick` _asbp_base_npc))
      (`KismetSystemLibrary.PrintString` "완전끝")
      (set `self.트레이스 변화 가능` true)
      ; 추적할 대상 삭제
      (set `self.추적할 NPC` null)
      (`KismetSystemLibrary.K2_ClearTimer` (stale `self.ReceiveTick` _asbp_base_npc) "플레이어 추적"))))

(fn `AI이동`
  (bind _controllednpc (`self.ControlledNPC`))
  (`self.MoveToActor` (`|GetArrayItem` (`/Game/Characters/NPC/BP_BaseNPC.순찰지점` _controllednpc) (`/Game/Characters/NPC/BP_BaseNPC.현재 순찰지점 인덱스` _controllednpc)) -1.0 true true true null))

(fn `NPC 행동양식 기록`
  (`KismetArrayLibrary.Array_Add` (`self.행동정수배열`) (`BlackboardComponent.GetValueAsInt` (`self.Blackboard`) (`self.랜덤 행동 정수`))))

(fn `UserConstructionScript`)

(fn `근접 적 추적 회전`)

(fn `적 추적`
  (params (`공격 범위` :type "Float (double-precision)"))
  (returns (NewParam :type "/Game/Characters/NPC/ENPCSTATE Enum"))
  (set `self.npc 상태` "NewEnumerator4")
  (bind _returnvalue (`self.MoveToActor` (`self.추적할 NPC`) `공격 범위` true true false null false))
  (switch `EPathFollowingRequestResult` _returnvalue
    (:`AlreadyAtGoal`
      (set `self.npc 상태` "NewEnumerator2"))
    (:`RequestSuccessful`
      (set `self.npc 상태` "NewEnumerator4")))
  (return (`self.npc 상태`)))