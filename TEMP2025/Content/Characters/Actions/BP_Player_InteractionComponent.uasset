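; Player interaction component that detects nearby interactable objects and reports them through event dispatchers meant for controller hookup.
; Overlap functions maintain NearbyActors and broadcast changes; while it is non-empty, Tick traces from the camera on the Camera channel.
; Trace reach varies with first- or third-person view, and the hit actor's name and type, read via message calls, are broadcast every frame.
; Interact and Highlight are empty stubs.
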(event `self.ReceiveTick`
  (params (DeltaSeconds :type "Float (single-precision)"))
  (if (`KismetArrayLibrary.Array_IsNotEmpty` (`self.NearbyActors`))
    (set `self.근처에 누구 있음 -> 컨트롤러 연결용` true)
    (bind (_hitactor _itype _name `_충돌있음`) (`self.LineTraceInteraction`))
    (`self.근처에 누구있는지 체크용 이벤트 디스패처` (`KismetStringLibrary.Conv_StringToName` _name) true _hitactor `_충돌있음` _itype)
    (`KismetSystemLibrary.PrintString` "as6d151")
    (else
      (set `self.근처에 누구 있음 -> 컨트롤러 연결용` false)
      (`self.근처에 누구있는지 체크용 이벤트 디스패처` "None"))))

(fn `Highlight`)

(fn `Interact`)

(fn `LineTraceInteraction`
  (returns (HitActor :type "Actor Object Reference") (Itype :type "EObjectType Enum") (Name :type String) (`충돌있음` :type Boolean))
  (bind _returnvalue (`GameplayStatics.GetPlayerCameraManager` 0))
  (bind _returnvalue_2 (`SceneComponent.K2_GetComponentLocation` (`Actor.RootComponent` _returnvalue)))
  ;[1 1 1] 입력 반응 -> 전달
  ;; 나중에 cast 말고 다르게
  (bind _asbp_first_person_character (cast `/Game/FirstPerson/Blueprints/BP_FirstPersonCharacter` (`GameplayStatics.GetPlayerPawn` 0)))
  (if (`/Game/FirstPerson/Blueprints/BP_FirstPersonCharacter.현재시점` _asbp_first_person_character)
    (set `self.1인칭3인칭상호작용거리` (300.0 300.0 300.0))
    (else
      (set `self.1인칭3인칭상호작용거리` (1200.0 1200.0 1200.0))))
  (bind (_outhit _returnvalue_3) (`KismetSystemLibrary.LineTraceSingle` _returnvalue_2 (+ _returnvalue_2 (* (`SceneComponent.GetForwardVector` (`Actor.RootComponent` _returnvalue)) (`self.1인칭3인칭상호작용거리`))) "TraceTypeQuery2"))
  (bind (_bblockinghit _binitialoverlap _time _distance _location _impactpoint _normal _impactnormal _physmat _hitactor) (`GameplayStatics.BreakHitResult` _outhit))
  (bind _name (message `/Game/Characters/Actions/BPI_NPC_OBJ.GetOBJName` _hitactor))
  (bind _newparam (message `/Game/Characters/Actions/BPI_NPC_OBJ.GetEOBJType` _hitactor "Misc"))
  (return _hitactor _newparam (`KismetTextLibrary.Conv_TextToString` _name) _returnvalue_3))

(fn `오버랩 발생 -> 컨트롤러연결`
  (params (NewParam :type "Actor Object Reference"))
  (`KismetArrayLibrary.Array_Add` (`self.NearbyActors`) NewParam)
  (`self.오버랩 체크용 디스패처` true))

(fn `오버랩 해제 -> 컨트롤러 해제`
  (params (NewParam :type "Actor Object Reference"))
  (`KismetArrayLibrary.Array_RemoveItem` (`self.NearbyActors`) NewParam)
  (`self.오버랩 체크용 디스패처` false))