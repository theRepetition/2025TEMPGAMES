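; BP_DodgeComponent is an actor component that gives its owning character a stamina-gated dodge.
; CanDodge requires no active dodge and more stamina in the owner's BP_StaminaComponent than the cost.
; ExecuteDodge spends stamina, flags dodging, delegates movement to the owner via MoveCharacterMessage and prints a debug string.
; A looping, near-instant timer calls ResetDodge, so the flag clears almost immediately and keeps being cleared.
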(fn `CanDodge`
  (returns (NewParam :type Boolean))
  (bind _newparam (`/Game/Characters/Actions/BP/BP_StaminaComponent.GetStamina` (`Actor.GetComponentByClass` (`self.GetOwner`) "/Game/Characters/Actions/BP/BP_StaminaComponent.BP_StaminaComponent_C")))
  (bind _output_get (set `self.CanDodgeV` (and (> _newparam (`self.StaminaCost`)) (== (`self.bIsDodging`) false))))
  (return _output_get))

(fn `Execute Dodge`
  (params (Dodgedirection :type "Vector Structure") (DodgeDistance :type "Float (double-precision)"))
  (bind _returnvalue (`self.GetOwner`))
  (bind _newparam (`self.CanDodge`))
  (if _newparam
    (`/Game/Characters/Actions/BP/BP_StaminaComponent.ReduceStamina` (`Actor.GetComponentByClass` _returnvalue "/Game/Characters/Actions/BP/BP_StaminaComponent.BP_StaminaComponent_C") (`self.StaminaCost`))
    (set `self.bIsDodging` true)
    (message `/Game/Characters/Actions/BP/BPI_DodgeInterface.MoveCharacter` _returnvalue Dodgedirection DodgeDistance)
    (`KismetSystemLibrary.K2_SetTimer` null "ResetDodge" 0.01 true)
    (`KismetSystemLibrary.PrintString` "회피!")))

(fn `ResetDodge`
  (set `self.bIsDodging` false))