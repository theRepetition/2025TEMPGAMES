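; Stamina component for action characters that tracks a clamped stamina pool, with combat-state setters and getters for current, maximum and percentage values.
; A looping timer regenerates stamina while recovery is enabled, using the tick amount modulo CombatRecoveryRate during combat.
; Draining stamina to zero halts recovery and starts a RecoverDelay timer.
; CanPerformAction ignores its Cost input, passing whenever stamina is above zero, and prints debug messages.
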(event `self.ReceiveBeginPlay`
  (`KismetSystemLibrary.K2_SetTimerDelegate` (delegate `RegenerateEvent`) 0.3 true))

(event `RegenerateEvent`
  (`self.RegenerateStamina` 5.0))

(event `EnableStaminaRecovery`
  (set `self.IsRecovering` true))

(fn `CanPerformAction`
  (params (Cost :type "Float (double-precision)"))
  (returns (Return :type Boolean))
  (bind _newparam (`self.GetStamina`))
  (`KismetSystemLibrary.PrintString` (`KismetStringLibrary.Conv_DoubleToString` _newparam))
  (bind _returnvalue (> _newparam 0.0))
  (if _returnvalue
    (return _returnvalue)
    (else
      (`KismetSystemLibrary.PrintString` "스태미나 낮음")
      (return _returnvalue))))

(fn `GetMaxStamina`
  (returns (NewParam :type "Float (double-precision)"))
  (return (`self.MAXstamina`)))

(fn `GetStamina`
  (returns (NewParam :type "Float (double-precision)"))
  (return (`self.Stamina`)))

(fn `GetStaminaPercent`
  (returns (Get :type "Float (double-precision)"))
  (return (/ (`self.Stamina`) (`self.MAXstamina`))))

(fn `OutofCombat`
  (set `self.IsInCombat` false))

(fn `ReduceStamina`
  (params (Amount :type "Float (double-precision)"))
  (bind _output_get (set `self.Stamina` (`KismetMathLibrary.FClamp` (- (`self.Stamina`) Amount) 0.0 (`self.MAXstamina`))))
  (if (<= _output_get 0.0)
    (set `self.IsRecovering` false)
    (`KismetSystemLibrary.K2_SetTimerDelegate` (`|CreateDelegate` :!event `EnableStaminaRecovery`) (`self.RecoverDelay`))))

(fn `RegenerateStamina`
  (params (Amount :type "Float (double-precision)"))
  (bind _stamina (`self.Stamina`))
  (bind _maxstamina (`self.MAXstamina`))
  (`self.GetStamina`)
  ;[1 1 1] 회복 가능 상태 확인
  (if (`self.IsRecovering`)
    ;[1 1 1] 전투상태 확인
    (if (`self.IsInCombat`)
      ;[1 1 1] 전투중일때
      (set `self.Stamina` (`KismetMathLibrary.FClamp` (+ (mod Amount (`self.CombatRecoveryRate`)) _stamina) 0.0 _maxstamina))
      (`KismetSystemLibrary.PrintString` "전투중")
      (else
        (set `self.Stamina` (`KismetMathLibrary.FClamp` (+ Amount _stamina) 0.0 _maxstamina))))))

(fn `SetCombat`
  (set `self.IsInCombat` true))