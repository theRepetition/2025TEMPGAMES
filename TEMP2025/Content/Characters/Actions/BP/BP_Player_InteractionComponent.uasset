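; Player interaction component that detects NPCs in front of the camera, still at a prototype stage.
; LineTraceInteraction traces a short distance forward from the player camera manager on the Camera channel, with persistent debug drawing.
; A hit actor tagged "NPC" only triggers an on-screen debug message.
; Interact, Highlight, BeginPlay and Tick are empty, and nothing in the component calls the trace.
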(fn `Highlight`)

(fn `Interact`)

(fn `LineTraceInteraction`
  (bind _returnvalue (`GameplayStatics.GetPlayerCameraManager` 0))
  (bind _returnvalue_2 (`SceneComponent.K2_GetComponentLocation` (`Actor.RootComponent` _returnvalue)))
  (bind (_outhit _returnvalue_3) (`KismetSystemLibrary.LineTraceSingle` :`Start` _returnvalue_2 :`End` (+ _returnvalue_2 (* (`SceneComponent.GetForwardVector` (`Actor.RootComponent` _returnvalue)) (300.0 300.0 300.0))) :`TraceChannel` "TraceTypeQuery2" :`DrawDebugType` "Persistent"))
  (if _returnvalue_3
    (if (`Actor.ActorHasTag` (`.HitActor` (`GameplayStatics.BreakHitResult` _outhit)) "NPC")
      (`KismetSystemLibrary.PrintString` "NPC상호작용"))))