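; BP_corpse is a world actor representing a dead NPC's body, holding a looting inventory.
; InitializeFromNPC stores the passed-in inventory and name, copies the source's skeletal mesh asset, and enables physics simulation on its own mesh.
; GetEOBJType returns a stored variable as the object type.
; The event graph holds only disabled default events, so the actor has no tick or overlap logic.
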(fn `GetEOBJType`
  (params (OBJTYPE :type "EObjectType Enum" :default "None"))
  (returns (NewParam :type "EObjectType Enum"))
  (return (`self.NewVar`)))

(fn `InitializeFromNPC`
  (params (NewParam :type "SkeletalMeshComponent Object Reference") (NewParam1 :type "Array of ItemData Structure") (NewParam2 :type String))
  (bind _skeletalmesh (`self.SkeletalMesh`))
  (set `self.루팅_인벤토리` NewParam1)
  (set `self.Name` NewParam2)
  (`SkeletalMeshComponent.SetSkeletalMeshAsset` _skeletalmesh (`SkeletalMeshComponent.GetSkeletalMeshAsset` NewParam))
  (`PrimitiveComponent.SetSimulatePhysics` _skeletalmesh true))

(fn `UserConstructionScript`
  (`parent.UserConstructionScript`))