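; Base NPC Blueprint with faction standing, damage and death handling, and short speech-bubble dialogue.
; BeginPlay loads profile, inventory and faction from data tables, then swaps in the GameInstance's matching runtime faction.
; ATKTOACTOR applies damage, lowers faction standing through the GameInstance for player attacks, and at zero health spawns a lootable BP_corpse.
; PlayertoNPC gets a relationship-based line from BPConversationComponent, shown in a widget for a text-length-scaled duration.
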(event `self.ReceiveBeginPlay`
  ;[1 1 1] npc 대화 지문 ui collapsed
  (set `Widget.Visibility` "Collapsed" (`WidgetComponent.GetUserWidgetObject` (`self.간단한대화위젯컴포넌트`)))
  ;[1 1 1] NPC 데이터 가져오기
  (bind _returnvalue (`|GetDataTableRow` "/Game/0_DataTable/DT_NPCDataTable.DT_NPCDataTable" (`self.NPCID`))
    (:`then`
      (bind _output_get (set `self.NPC 정보` _returnvalue))
      (bind (`_팩션` `_npc타입` `_클래스` `_아이템테이블` `_프로필`) (break `/Game/0_DataTable/bp_NpcStruct` _output_get))
      (bind _output_get_2 (set `self.프로필` `_프로필`))
      (set `self.NPC 인벤토리` `_아이템테이블`)
      (bind (_playername _level _health) (break `PlayerProfile` _output_get_2))
      (set `self.Name` _playername)
      (bind _output_get_3 (set `self.MaxHealth` _health))
      (set `self.Health` _output_get_3)
      (bind _returnvalue_2 (`|GetDataTableRow` "/Game/0_DataTable/DT_FAactionDataTable.DT_FAactionDataTable" `_팩션`)
        (:`then`
          (bind _output_get_4 (set `self.Faction` _returnvalue_2))
          ;;[1 1 1] 팩션 같은거 있을때만 인스턴스 관계도 수치 받아오기
          (bind _asbp_game_instance (cast `/Game/0_Game/BP_GameInstance` (`GameplayStatics.GetGameInstance`)))
          (for _array_element (`/Game/0_Game/BP_GameInstance.팩션` _asbp_game_instance)
            (if (== (`.팩션이름_9_0F6684564B773AA659EC06B9743BF796` (break `/Game/0_DataTable/bp_FactionStruct` _output_get_4)) (`.팩션이름_9_0F6684564B773AA659EC06B9743BF796` (break `/Game/0_DataTable/bp_FactionStruct` _array_element)))
              (set `self.Faction` _array_element))))))))

(event `/Game/0_Characters/NPC/BPI_ATKTO.ATKTOACTOR`
  (params (`공격구조체` :type "/Game/FirstPerson/Blueprints/Attack/bp_ATKSTRucture Structure") (`공격자` :type "Actor Object Reference"))
  (bind (`_기본데미지` `_공격타입` `_공격방향`) (break `/Game/FirstPerson/Blueprints/Attack/bp_ATKSTRucture` `공격구조체`))
  (bind _health (`self.Health`))
  (bind _faction (`self.Faction`))
  (bind (`_팩션이름` `_플레이어와의관계수치`) (break `/Game/0_DataTable/bp_FactionStruct` _faction))
  (set `self.피해 받았는지 체크` true)
  ;[1 1 1] 피해 입는 판정
  (`KismetSystemLibrary.PrintString` (`|GetEnumeratorNameAsString` `_공격방향`))
  (set `self.Health` (- _health `_기본데미지`))
  ;[1 1 1 1 12] 플레이어가 공격했으면 해당 팩션의 관계도를 낮추기
  ; 데이터를 건드는게 아니라
  ; 인스턴스하고 연결해서 인스턴스 내부의 현재 게임의 관계도를 설정해야함
  (cast `/Game/FirstPerson/Blueprints/BP_FirstPersonCharacter` `공격자`
    (:`then`
      (bind _asbp_game_instance (cast `/Game/0_Game/BP_GameInstance` (`GameplayStatics.GetGameInstance`)))
      (setmembers `/Game/0_DataTable/bp_FactionStruct` :`StructRef` _faction :`플레이어와의 관계 수치` (- `_플레이어와의관계수치` 1))
      (`KismetSystemLibrary.PrintString` (`KismetStringLibrary.Conv_IntToString` `_플레이어와의관계수치`))
      (`/Game/0_Game/BP_GameInstance.팩션 관계도 감소` _asbp_game_instance _faction))
    (:`CastFailed`
      _))
  ;[1 1 1] 사망 처리후 시체 파밍
  (if (<= _health 0.0)
    (bind _returnvalue (`|SpawnActorFromClass` "/Game/World/BP_corpse.BP_corpse_C" (`SceneComponent.GetSocketTransform` (`self.Mesh`) "Root" "RTS_World") "AdjustIfPossibleButAlwaysSpawn" "MultiplyWithRoot" null null))
    (`/Game/World/BP_corpse.InitializeFromNPC` _returnvalue (`self.Mesh`) (`self.NPC 인벤토리`) (`self.Name`))
    (`self.K2_DestroyActor`)
    (set `self.사망처리` true)
    (else
      (`KismetSystemLibrary.Delay` 0.2)
      (set `self.피해 받았는지 체크` false))))

(event `/Game/0_Characters/Actions/BPI_NPCInteraction.PlayertoNPC`
  (params (NewParam :type "/Game/0_Characters/Actions/STR_PlayerToNPC Structure"))
  (bind (_playername _test_str) (break `/Game/0_Characters/Actions/STR_PlayerToNPC` NewParam))
  (`cppNPCInteraction.ProcessPlayerStateWithValue` (`self.cppNPCInteraction`) _playername _test_str 0)
  (bind `_출력_짧은_대화문` (`/Game/0_Characters/NPC/BP_ConversationComponent.대화시작` (`self.BP_ConversationComponent`) (`.플레이어와의관계수치_6_56E833414AD9AE5DB1DCE088D8325AE9` (break `/Game/0_DataTable/bp_FactionStruct` (`self.Faction`))) (`self.Name`) (`self.긴대화지문가지고있음`)))
  (`self.간단한 대화문 출력` (`KismetTextLibrary.Conv_StringToText` `_출력_짧은_대화문`)))

(event `간단한 대화문 출력`
  (params (`간단한 대화문 텍스트 입력` :type Text))
  (bind _returnvalue (`WidgetComponent.GetUserWidgetObject` (`self.간단한대화위젯컴포넌트`)))
  (bind _aswbp_speech_box (cast `/Game/UI/WBP_SpeechBox` _returnvalue))
  (`/Game/UI/WBP_SpeechBox.set짧은대화지문` _aswbp_speech_box `간단한 대화문 텍스트 입력`)
  (`Widget.SetVisibility` _returnvalue "Visible")
  (`KismetSystemLibrary.Delay` (+ (* (`self.NewVar`) (`KismetStringLibrary.Len` (`KismetTextLibrary.Conv_TextToString` `간단한 대화문 텍스트 입력`))) 2.0))
  (`Widget.SetVisibility` _returnvalue "Collapsed"))

(fn `GetEOBJType`
  (params (OBJTYPE :type "EObjectType Enum" :default "None"))
  (returns (NewParam :type "EObjectType Enum"))
  (return (`self.OBJTYPE`)))

(fn `GetOBJName`
  (returns (name :type Text))
  (return (`KismetTextLibrary.Conv_StringToText` (`self.Name`))))

(fn `UserConstructionScript`)