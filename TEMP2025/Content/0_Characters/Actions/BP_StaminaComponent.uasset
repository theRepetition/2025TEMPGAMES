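; Stamina component for the first-person character that tracks stamina, gates actions on it and exposes it as a percentage.
; A looping timer regenerates stamina while recovery is allowed, capped by the owner's PlayerProfile maximum.
; Draining stamina to zero halts recovery and starts a delay timer.
; In combat, regeneration adds the amount modulo CombatRecoveryRate (a remainder, not a scaled rate) instead of the full amount.
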(event `self.ReceiveBeginPlay`
  (`KismetSystemLibrary.K2_SetTimerDelegate` (delegate `RegenerateEvent`) 0.3 true))

(event `RegenerateEvent`
  (bind _asbp_first_person_character (cast `/Game/FirstPerson/Blueprints/BP_FirstPersonCharacter` (`self.GetOwner`)))
  (`self.RegenerateStamina` 5.0 (`.Stamina` (break `PlayerProfile` (`/Game/FirstPerson/Blueprints/BP_FirstPersonCharacter.PlayerProfile` _asbp_first_person_character)))))

(event `EnableStaminaRecovery`
  (set `self.IsRecovering` true))

(fn `CanPerformAction`
  (params (stamina :type "Float (double-precision)"))
  (returns (Return :type Boolean))
  (bind _returnvalue (> (`self.Stamina`) 0.0))
  (if _returnvalue
    (return _returnvalue)
    (else
      (`KismetSystemLibrary.PrintString` "스태미나 낮음")
      (return _returnvalue))))

(fn `GetMaxStamina`
  (returns (NewParam :type "Float (double-precision)"))
  (return (`self.MAXstamina`)))

(fn `GetStamina`
  (returns (NewParam :type "Float (double-precision)"))
  (return (`self.Stamina`)))

(fn `GetStaminaPercent`
  (params (MAXstamina :type "Float (double-precision)"))
  (returns (Get :type "Float (double-precision)"))
  (return (/ (`self.Stamina`) MAXstamina)))

(fn `OutofCombat`
  (set `self.IsInCombat` false))

(fn `ReduceStamina`
  (params (Amount :type "Float (double-precision)") (MaxStamina :type "Float (double-precision)"))
  (bind _output_get (set `self.Stamina` (`KismetMathLibrary.FClamp` (- (`self.Stamina`) Amount) 0.0 MaxStamina)))
  (if (<= _output_get 0.0)
    (set `self.IsRecovering` false)
    (`KismetSystemLibrary.K2_SetTimerDelegate` (`|CreateDelegate` :!event `EnableStaminaRecovery`) (`self.RecoverDelay`))))

(fn `RegenerateStamina`
  (params (Amount :type "Float (double-precision)") (maxstamina :type "Float (double-precision)"))
  (bind _stamina (`self.Stamina`))
  (`self.GetStamina`)
  ;[1 1 1] 회복 가능 상태 확인
  (if (`self.IsRecovering`)
    ;[1 1 1] 전투상태 확인
    (if (`self.IsInCombat`)
      ;[1 1 1] 전투중일때
      (set `self.Stamina` (`KismetMathLibrary.FClamp` (+ (mod Amount (`self.CombatRecoveryRate`)) _stamina) 0.0 maxstamina))
      (`KismetSystemLibrary.PrintString` "전투중")
      (else
        (set `self.Stamina` (`KismetMathLibrary.FClamp` (+ Amount _stamina) 0.0 maxstamina))))))

(fn `SetCombat`
  (set `self.IsInCombat` true))