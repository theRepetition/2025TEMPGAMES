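; Player interaction component that finds the object the player's camera is looking at.
; LineTraceInteraction casts a short Camera-channel ray forward from the player camera manager and queries the hit actor for its object name and type via messages.
; It returns the actor, type, name and hit flag to the caller.
; Interact and Highlight are empty stubs, and the event graph has no logic.
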(fn `Highlight`)

(fn `Interact`)

(fn `LineTraceInteraction`
  (returns (HitActor :type "Actor Object Reference") (Itype :type "EObjectType Enum") (Name :type String) (`충돌있음` :type Boolean))
  (bind _returnvalue (`GameplayStatics.GetPlayerCameraManager` 0))
  (bind _returnvalue_2 (`SceneComponent.K2_GetComponentLocation` (`Actor.RootComponent` _returnvalue)))
  ;[1 1 1] 입력 반응 -> 전달
  (bind (_outhit _returnvalue_3) (`KismetSystemLibrary.LineTraceSingle` _returnvalue_2 (+ _returnvalue_2 (* (`SceneComponent.GetForwardVector` (`Actor.RootComponent` _returnvalue)) (300.0 300.0 300.0))) "TraceTypeQuery2"))
  (bind (_bblockinghit _binitialoverlap _time _distance _location _impactpoint _normal _impactnormal _physmat _hitactor) (`GameplayStatics.BreakHitResult` _outhit))
  (bind _name (message `/Game/0_Characters/Actions/BPI_NPC_OBJ.GetOBJName` _hitactor))
  (bind _newparam (message `/Game/0_Characters/Actions/BPI_NPC_OBJ.GetEOBJType` _hitactor "Misc"))
  (return _hitactor _newparam (`KismetTextLibrary.Conv_TextToString` _name) _returnvalue_3))