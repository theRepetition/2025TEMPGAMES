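; BP_Itemcomponent is an item component that holds an item's instance identity and supplies its data as an inventory entry.
; On BeginPlay, 아이템생성스폰 (item create/spawn) sets the instance ID, keeping a valid passed-in GUID or generating a new one, as happens here.
; A separate function builds a single-quantity inventory entry from the current item's definition ID, name and X/Y grid size.
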(event `self.ReceiveBeginPlay`
  (`self.아이템 생성/스폰` (struct)))

(fn `아이템 생성/스폰`
  (params (NewParam :type "Guid Structure"))
  (bind `_아이템_인스턴스` (`self.아이템 인스턴스`))
  (if (`KismetGuidLibrary.IsValid_Guid` NewParam)
    (setmembers `/Game/Items/Item_InstanceID` :`StructRef` `_아이템_인스턴스` :`Instance ID` NewParam)
    (else
      (setmembers `/Game/Items/Item_InstanceID` :`StructRef` `_아이템_인스턴스` :`Instance ID` (`KismetGuidLibrary.NewGuid`)))))

(fn `아이템 정보 인스턴스 생성후 전달`
  (returns (NewParam :type "/Game/Items/Item_InventoryEntry Structure"))
  (bind (_def_id _name _type _value _weight _quantity _x _y) (break `ItemData` (`self.현재 아이템`)))
  (return (make `/Game/Items/Item_InventoryEntry` "00000000000000000000000000000000" _def_id (`KismetStringLibrary.Conv_StringToName` _name) 1 0 0 false _x _y)))